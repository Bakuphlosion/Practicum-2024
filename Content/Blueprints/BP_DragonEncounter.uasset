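; BP_DragonEncounter is a box trigger that starts the dragon battle.
; On overlap, it checks RPInstance, proceeding only if the dragon is not down and HasMilk is set.
; It then flags DragonBattle on the game instance, calls SetIgnoreMoveInput with false, and shows a W_Textbox attack message.
; After a short delay it opens the BattleScreen level.
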(event OnComponentBeginOverlap(Box)
  (params (OverlappedComponent :type Primitive%20Component%20Object%20Reference) (OtherActor :type Actor%20Object%20Reference) (OtherComp :type Primitive%20Component%20Object%20Reference) (OtherBodyIndex :type Integer) (bFromSweep :type Boolean) (SweepResult :type Hit%20Result%20Structure%20%28by%20ref%29))
  (bind _asrpinstance (Utilities|Casting|CastToRPInstance (Game|GetGameInstance)))
  (if (not (Variables|/Game/RPInstance.RPInstance_C|GetDragonDown _asrpinstance))
    (if (Variables|/Game/RPInstance.RPInstance_C|GetHasMilk _asrpinstance)
      (Variables|/Game/RPInstance.RPInstance_C|SetDragonBattle _asrpinstance true)
      (Input|SetIgnoreMoveInput (Game|GetPlayerController 0) false)
      (bind _returnvalue (UserInterface|CreateWidget "/Game/UserInterface/BattleUI/W_Textbox.W_Textbox_C"))
      (UserInterface|Viewport|AddtoViewport _returnvalue 0)
      (Rendering|Components|TextRender|SetText (Variables|/Game/UserInterface/BattleUI/W_Textbox.W_Textbox_C|GetTextboxText _returnvalue) "A dragon suddenly attacks!")
      (Utilities|FlowControl|Delay 3.0)
      (Game|OpenLevel(byObjectReference) "/Game/Levels/BattleScreen.BattleScreen"))))

(fn ConstructionScript)