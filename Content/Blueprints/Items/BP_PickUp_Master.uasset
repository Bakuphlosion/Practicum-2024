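; BP_PickUp_Master is a pickup actor, named as a master, that adds an item to the player's inventory.
; Its construction script applies the PickUpMesh and Material variables to the Cube component, so each pickup's look is configurable.
; When BP_ThirdPersonCharacter overlaps it, it adds its Type to the Inventory stored on the RPInstance game instance, then destroys itself.
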(event Collision|EventActorBeginOverlap
  (params (OtherActor :type Actor%20Object%20Reference))
  (Utilities|Casting|CastToBP_ThirdPersonCharacter OtherActor)
  (bind _asrpinstance (Utilities|Casting|CastToRPInstance (Game|GetGameInstance)))
  (Utilities|Array|Add (Variables|/Game/RPInstance.RPInstance_C|GetInventory _asrpinstance) (Variables|Default|GetType))
  (Actor|DestroyActor))

(fn ConstructionScript
  (Components|StaticMesh|SetStaticMesh (Variables|Default|GetCube) (Variables|Default|GetPickUpMesh))
  (Rendering|Material|SetMaterial (Variables|Default|GetCube) 0 (Variables|Default|GetMaterial)))