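; Overworld enemy that wanders the level, chases a player it sees and starts a battle on contact.
; Tick alternates random AI moves with pursuit triggered by PawnSensing.
; Box overlap fades the camera, saves enemy number, level and player location to RPInstance, then opens BattleScreen.
; On BeginPlay it destroys itself if RPInstance marks it defeated, otherwise it ignores contact briefly before clearing the stored enemy number.
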(event OnComponentBeginOverlap(Box)
  (params (OverlappedComponent :type Primitive%20Component%20Object%20Reference) (OtherActor :type Actor%20Object%20Reference) (OtherComp :type Primitive%20Component%20Object%20Reference) (OtherBodyIndex :type Integer) (bFromSweep :type Boolean) (SweepResult :type Hit%20Result%20Structure%20%28by%20ref%29))
  ;[1 1 1] When touching, begin battle
  (if (Variables|Default|GetInvincibility)
    (Development|PrintString " ")
    (else
      (bind _asrpinstance (Utilities|Casting|CastToRPInstance (Game|GetGameInstance)))
      (bind _asbp_third_person_character (Utilities|Casting|CastToBP_ThirdPersonCharacter (Game|GetPlayerCharacter 0)))
      (Variables|Default|SetCaughtPlayer true)
      (Audio|PlaySound2D "/Game/Sounds/SFX/Enemy_Encounter.Enemy_Encounter" 1.0 1.0 0.0 0 0)
      (Input|SetIgnoreMoveInput (Game|GetPlayerController 0) false)
      (CameraFades|StartCameraFade :self (Game|GetPlayerCameraManager 0) :ToAlpha 1.0 :Duration 1.0 :bHoldWhenFinished true)
      (Utilities|FlowControl|Delay 1.0)
      (Variables|/Game/RPInstance.RPInstance_C|SetEnemyNo _asrpinstance (Variables|Default|GetEnemyNumber))
      (bind _returnvalue (Game|GetCurrentLevelName true))
      (Variables|/Game/RPInstance.RPInstance_C|SetCurrent%20Level _asrpinstance _returnvalue)
      (Variables|/Game/RPInstance.RPInstance_C|SetPlayerLocation _asrpinstance (Transformation|GetActorLocation _asbp_third_person_character))
      (Game|OpenLevel(byObjectReference) "/Game/Levels/BattleScreen.BattleScreen"))))

(event OnSeePawn(PawnSensing)
  (params (Pawn :type Pawn%20Object%20Reference))
  (Variables|Default|SetSeesPlayer true)
  (bind _asbp_third_person_character (Utilities|Casting|CastToBP_ThirdPersonCharacter Pawn))
  (CallFunction|FollowPlayer))

(event Custom|FollowPlayer
  (AI|AIMoveTo self "0, 0, 0" (stale OnSeePawn(PawnSensing) _asbp_third_person_character) 5.0 false
    (:then
      (Utilities|FlowControl|Delay 5.0))
    (:OnSuccess
      _))
  (Variables|Default|SetSeesPlayer false))

(event EventBeginPlay
  (Variables|Default|SetInvincibility true)
  (bind _asrpinstance (Utilities|Casting|CastToRPInstance (Game|GetGameInstance)))
  (if (Variables|/Game/RPInstance.RPInstance_C|GetEnemyDefeated _asrpinstance)
    (if (== (Variables|/Game/RPInstance.RPInstance_C|GetEnemyNo _asrpinstance) (Variables|Default|GetEnemyNumber))
      (Actor|DestroyActor)
      (else
        (Utilities|FlowControl|Delay 2.0 :!label _label)
        (Variables|Default|SetInvincibility false)
        (Variables|/Game/RPInstance.RPInstance_C|SetEnemyNo _asrpinstance -1)))
    (else
      (goto _label))))

(event EventTick
  (params (DeltaSeconds :type Float%20%28single-precision%29))
  (if (not (Variables|Default|GetCaughtPlayer))
    (if (Variables|Default|GetSeesPlayer)
      (CallFunction|FollowPlayer)
      (else
        (Utilities|FlowControl|Delay (Math|Random|RandomFloatinRange 1.0 5.0))
        (AI|AIMoveTo self (.RandomLocation (AI|Navigation|GetRandomReachablePointinRadius (Transformation|GetActorLocation) 1e+03 0 0)) 0 5.0 false)))))

(fn ConstructionScript)