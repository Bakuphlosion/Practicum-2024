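; BP_EnemyReal is an overworld enemy that chases the player and starts a battle on contact.
; On BeginPlay it destroys itself if the RPInstance game instance marks EnemyDefeated, otherwise it drops a short invincibility window after a delay.
; PawnSensing moves it toward a seen BP_ThirdPersonCharacter with AIMoveTo.
; A Box overlap opens the BattleScreen level unless still invincible, without filtering the overlapping actor.
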(event OnComponentBeginOverlap(Box)
  (params (OverlappedComponent :type Primitive%20Component%20Object%20Reference) (OtherActor :type Actor%20Object%20Reference) (OtherComp :type Primitive%20Component%20Object%20Reference) (OtherBodyIndex :type Integer) (bFromSweep :type Boolean) (SweepResult :type Hit%20Result%20Structure%20%28by%20ref%29))
  ;[1 1 1] When touching, begin battle
  (if (Variables|Default|GetInvincible)
    (Development|PrintString " ")
    (else
      (Game|OpenLevel(byObjectReference) "/Game/Levels/BattleScreen.BattleScreen"))))

(event OnSeePawn(PawnSensing)
  (params (Pawn :type Pawn%20Object%20Reference))
  (bind _asbp_third_person_character (Utilities|Casting|CastToBP_ThirdPersonCharacter Pawn))
  (AI|AIMoveTo self (Transformation|GetActorLocation _asbp_third_person_character) (Game|GetPlayerCharacter 0) 5.0 false))

(event EventBeginPlay
  (Variables|Default|SetInvincible true)
  (bind _asrpinstance (Utilities|Casting|CastToRPInstance (Game|GetGameInstance)))
  (if (Variables|/Game/RPInstance.RPInstance_C|GetEnemyDefeated _asrpinstance)
    (Actor|DestroyActor)
    (else
      (Utilities|FlowControl|Delay 2.0)
      (Variables|Default|SetInvincible false))))

(fn ConstructionScript)