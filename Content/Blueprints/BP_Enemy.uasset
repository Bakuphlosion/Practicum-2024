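; BP_Enemy is an enemy actor that opens a battle level on overlap and holds the enemy's combat logic.
; On BeginPlay it rolls stats in tiers by the game instance Score, then destroys itself if already flagged defeated or drops invincibility after a short delay.
; EnemyTurn subtracts player defense minus enemy attack, plus a random bonus, from player health.
; Turn, death and defeat flags are written to RPInstance.
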(event OnComponentBeginOverlap(Box)
  (params (OverlappedComponent :type Primitive%20Component%20Object%20Reference) (OtherActor :type Actor%20Object%20Reference) (OtherComp :type Primitive%20Component%20Object%20Reference) (OtherBodyIndex :type Integer) (bFromSweep :type Boolean) (SweepResult :type Hit%20Result%20Structure%20%28by%20ref%29))
  ;[1 1 1] When touching, begin battle
  (if (Variables|Default|GetInvincibility)
    (Development|PrintString " ")
    (else
      (Game|OpenLevel(byObjectReference) "/Game/Levels/BattleScreen.BattleScreen"))))

(event Custom|Enemy%20Turn
  (Audio|PlaySound2D "/Game/Sounds/Enemy_Hit.Enemy_Hit" 1.0 1.0 0.0 0 0)
  (bind _asrpinstance (Utilities|Casting|CastToRPInstance (Game|GetGameInstance)))
  (Variables|/Game/RPInstance.RPInstance_C|SetPlayerTurn _asrpinstance false)
  (Variables|Default|SetEnemyDamage (+ (- (Variables|/Game/RPInstance.RPInstance_C|GetPlayerDefense _asrpinstance) (Variables|Default|GetEnemyAtk)) (Math|Random|RandomIntegerinRange 0 3)))
  (Variables|/Game/RPInstance.RPInstance_C|SetPlayerHealth _asrpinstance (- (Variables|/Game/RPInstance.RPInstance_C|GetPlayerHealth _asrpinstance) (Variables|Default|GetEnemyDamage)))
  (if (<= (Variables|/Game/RPInstance.RPInstance_C|GetPlayerHealth _asrpinstance) 0)
    (Variables|/Game/RPInstance.RPInstance_C|SetPlayerDied _asrpinstance true)))

(event Custom|Enemy%20Defeated
  (bind _asrpinstance (Utilities|Casting|CastToRPInstance (Game|GetGameInstance)))
  (if (<= (Variables|Default|GetEnemyHP) 0)
    (Variables|Default|SetEnemyDead true)
    (Variables|/Game/RPInstance.RPInstance_C|SetEnemyDefeated _asrpinstance true)
    (else
      (Development|PrintString ""))))

(event EventBeginPlay
  (bind _asrpinstance (Utilities|Casting|CastToRPInstance (Game|GetGameInstance)))
  (if (<= (Variables|/Game/RPInstance.RPInstance_C|GetScore _asrpinstance) 5)
    (Variables|Default|SetEnemyHP (Math|Random|RandomIntegerinRange 5 10))
    (Variables|Default|SetEnemyAtk (Math|Random|RandomIntegerinRange 0 3))
    (Variables|Default|SetEnemyDef (Math|Random|RandomIntegerinRange 0 3))
    (Variables|Default|SetEnemySpd (Math|Random|RandomIntegerinRange 0 7))
    (elif (<= (Variables|/Game/RPInstance.RPInstance_C|GetScore _asrpinstance) 10)
      (Variables|Default|SetEnemyHP (Math|Random|RandomIntegerinRange 5 15))
      (Variables|Default|SetEnemyAtk (Math|Random|RandomIntegerinRange 2 5))
      (Variables|Default|SetEnemyDef (Math|Random|RandomIntegerinRange 2 5))
      (Variables|Default|SetEnemySpd (Math|Random|RandomIntegerinRange 3 9))
      (elif (<= (Variables|/Game/RPInstance.RPInstance_C|GetScore _asrpinstance) 15)
        (Variables|Default|SetEnemyHP (Math|Random|RandomIntegerinRange 10 20))
        (Variables|Default|SetEnemyAtk (Math|Random|RandomIntegerinRange 3 6))
        (Variables|Default|SetEnemyDef (Math|Random|RandomIntegerinRange 3 6))
        (Variables|Default|SetEnemySpd (Math|Random|RandomIntegerinRange 7 11))
        (elif (<= (Variables|/Game/RPInstance.RPInstance_C|GetScore _asrpinstance) 20)
          (Variables|Default|SetEnemyHP (Math|Random|RandomIntegerinRange 15 25))
          (Variables|Default|SetEnemyAtk (Math|Random|RandomIntegerinRange 5 8))
          (Variables|Default|SetEnemyDef (Math|Random|RandomIntegerinRange 5 8))
          (Variables|Default|SetEnemySpd (Math|Random|RandomIntegerinRange 9 13))
          (else
            (Variables|Default|SetEnemyHP (Math|Random|RandomIntegerinRange 5 30))
            (Variables|Default|SetEnemyAtk (Math|Random|RandomIntegerinRange 0 10))
            (Variables|Default|SetEnemyDef (Math|Random|RandomIntegerinRange 0 10))
            (Variables|Default|SetEnemySpd (Math|Random|RandomIntegerinRange 0 20)))))))
  (Variables|Default|SetInvincibility true)
  (bind _asrpinstance_2 (Utilities|Casting|CastToRPInstance (Game|GetGameInstance)))
  (if (Variables|/Game/RPInstance.RPInstance_C|GetEnemyDefeated _asrpinstance_2)
    (Actor|DestroyActor)
    (else
      (Utilities|FlowControl|Delay 2.0)
      (Variables|Default|SetInvincibility false))))

(fn ConstructionScript)