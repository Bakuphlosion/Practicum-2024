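; BP_NewLevel is a trigger box that handles level transitions, with special handling for the final room.
; On overlap it locks player movement, saves the current level name to the RPInstance game instance and plays a progression sound.
; It then fades the camera out and opens the configured Level by name.
; If FinalRoom is set and the instance has HasMilk, it only fades out, without loading a level.
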(event OnComponentBeginOverlap(Box)
  (params (OverlappedComponent :type Primitive%20Component%20Object%20Reference) (OtherActor :type Actor%20Object%20Reference) (OtherComp :type Primitive%20Component%20Object%20Reference) (OtherBodyIndex :type Integer) (bFromSweep :type Boolean) (SweepResult :type Hit%20Result%20Structure%20%28by%20ref%29))
  (bind _returnvalue (Game|GetPlayerCameraManager 0))
  (bind _returnvalue_2 (Game|GetPlayerCameraManager 0))
  (Input|SetIgnoreMoveInput (Game|GetPlayerController 0) true)
  (bind _asrpinstance (Utilities|Casting|CastToRPInstance (Game|GetGameInstance)))
  (bind _returnvalue_3 (Game|GetCurrentLevelName true))
  (Variables|/Game/RPInstance.RPInstance_C|SetCurrent%20Level _asrpinstance _returnvalue_3)
  (Audio|PlaySound2D "/Game/Sounds/SFX/Progression.Progression" 1.0 1.0 0.0 0 0)
  (if (Variables|Default|GetFinalRoom)
    (if (Variables|/Game/RPInstance.RPInstance_C|GetHasMilk _asrpinstance)
      (CameraFades|StartCameraFade :self _returnvalue_2 :ToAlpha 1.0 :Duration 0.8)
      (Utilities|FlowControl|Delay 0.8)
      (CameraFades|StartCameraFade :self _returnvalue_2 :FromAlpha 1.0 :ToAlpha 1.0 :Duration 0.5)
      (else
        (CameraFades|StartCameraFade :self _returnvalue :ToAlpha 1.0 :Duration 0.8 :!label _label)
        (Utilities|FlowControl|Delay 0.8)
        (CameraFades|StartCameraFade :self _returnvalue :FromAlpha 1.0 :ToAlpha 1.0 :Duration 0.5)
        (Game|OpenLevel(byName) (Utilities|String|StringToName (Variables|Default|GetLevel)))))
    (else
      (goto _label))))

(fn ConstructionScript)