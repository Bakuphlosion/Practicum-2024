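; BP_NextStage is a trigger box that advances the run to the next level when anything overlaps it.
; On overlap it increments Score on the RPInstance game instance, saves the high score and clears EnemyDefeated.
; It then opens RestStop when the score hits one of four fixed milestones at every fifth stage up to twenty, otherwise FightChamber.
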(event OnComponentBeginOverlap(Box)
  (params (OverlappedComponent :type Primitive%20Component%20Object%20Reference) (OtherActor :type Actor%20Object%20Reference) (OtherComp :type Primitive%20Component%20Object%20Reference) (OtherBodyIndex :type Integer) (bFromSweep :type Boolean) (SweepResult :type Hit%20Result%20Structure%20%28by%20ref%29))
  (bind _asrpinstance (Utilities|Casting|CastToRPInstance (Game|GetGameInstance)))
  (bind _result (Math|Integer|IncrementInt (Variables|/Game/RPInstance.RPInstance_C|GetScore _asrpinstance))
    (:%20%20
      (Default|SaveHighScore _asrpinstance)
      (Variables|/Game/RPInstance.RPInstance_C|SetEnemyDefeated _asrpinstance false)
      (if (Math|Boolean|ORBoolean (== _result 5) (== _result 10) (== _result 15) (== _result 20))
        (Game|OpenLevel(byObjectReference) "/Game/Levels/OldMinigame/RestStop.RestStop")
        (else
          (Game|OpenLevel(byObjectReference) "/Game/Levels/OldMinigame/FightChamber.FightChamber"))))))

(fn ConstructionScript)